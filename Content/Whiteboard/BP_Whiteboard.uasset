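; Whiteboard that can be drawn on with hit results, with the drawing saved and restored.
; BeginPlay creates a render target, shows it on the board mesh through a dynamic material, then loads the saved drawing.
; DrawLine converts hit collision UVs into canvas lines and records points in an array, with negative sentinels separating strokes.
; SaveBoard stores that array through DataSaveLoader, and LoadBoard replays it as lines using the current brush settings.
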(event EventBeginPlay
  (bind _returnvalue (Rendering|CreateRenderTarget2D 512 512 "RTF_RGBA16f" "(R=1.000000,G=1.000000,B=1.000000,A=1.000000)"))
  (bind _output_get (Variables|Default|SetRenderTarget _returnvalue))
  (Rendering|ClearRenderTarget2D _output_get (Variables|Default|GetInitialColor))
  (bind _returnvalue_2 (Rendering|Material|CreateDynamicMaterialInstance "/Game/Whiteboard/Material/M_RenderTarget.M_RenderTarget" "None" "None" :!class /Script/Engine.KismetMaterialLibrary))
  (Variables|Default|SetRTMatInstance _returnvalue_2)
  (Rendering|Material|SetTextureParameterValue _returnvalue_2 "RenderTarget" (Variables|Default|GetRenderTarget))
  (Rendering|Material|SetMaterial (Variables|Default|GetWhiteboard) 0 (Variables|Default|GetRTMatInstance))
  (CallFunction|LoadBoard))

(fn ConstructionScript)

(fn DrawLine
  (params (Hit :type Hit%20Result%20Structure) (InitHit :type Boolean))
  (bind _uv (Class|GameplayStatics|FindCollisionUV Hit))
  (if InitHit
    (Variables|Default|SetPrevHitUVLoc (* _uv (Variables|Default|GetBoardResolution)))
    (Utilities|Array|Add (Variables|Default|GetDrawArray) "(X=-1.000000,Y=-1.000000)")
    (else
      (bind (_canvas _size _context) (Rendering|BeginDrawCanvastoRenderTarget (Variables|Default|GetRenderTarget)))
      (Class|Canvas|DrawLine _canvas (Variables|Default|GetPrevHitUVLoc) (* _size _uv) (Variables|Default|GetBrushThickness) (Variables|Default|GetDrawColor))
      (Rendering|EndDrawCanvastoRenderTarget _context)
      (if (not (Math|Float|NearlyEqual(Float) (Math|Vector|Distance2D(Vector) (Variables|Default|GetPrevHitUVLoc) (* _size _uv)) 0.0 1e-06))
        (bind _output_get (Variables|Default|SetPrevHitUVLoc (* _size _uv)))
        (Utilities|Array|Add (Variables|Default|GetDrawArray) _output_get)))))

(fn ClearBoard
  (Rendering|ClearRenderTarget2D (Variables|Default|GetRenderTarget) (Variables|Default|GetInitialColor))
  (Utilities|Array|Clear (Variables|Default|GetDrawArray)))

(fn LoadBoard
  (CallFunction|ClearBoard)
  (Variables|Default|SetPrevDraw "")
  (bind _output_get (Variables|Default|SetDrawArray (Class|DataSaveLoader|LoadVec2Arr (Variables|Default|GetDataSaveLoader))))
  (Variables|Default|SetLoadFirst true)
  (for _array_element _output_get
    (if (> (.X (Math|Vector2D|BreakVector2D _array_element)) 0.0)
      (if (Variables|Default|GetLoadFirst)
        (Variables|Default|SetPrevDraw _array_element)
        (Variables|Default|SetLoadFirst false)
        (else
          (bind (_canvas _size _context) (Rendering|BeginDrawCanvastoRenderTarget (Variables|Default|GetRenderTarget)))
          (Class|Canvas|DrawLine _canvas (Variables|Default|GetPrevDraw) _array_element (Variables|Default|GetBrushThickness) (Variables|Default|GetDrawColor))
          (Rendering|EndDrawCanvastoRenderTarget _context)
          (Variables|Default|SetPrevDraw _array_element)))
      (else
        (Variables|Default|SetLoadFirst true)))))

(fn SaveBoard
  (Class|DataSaveLoader|SaveVec2Arr (Variables|Default|GetDataSaveLoader) (Variables|Default|GetDrawArray)))