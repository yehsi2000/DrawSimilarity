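; BP_DrawingComparer scores how similar the drawings on two whiteboards are and displays the results as text.
; RefreshText copies each board's DrawArray and, if both contain points, writes SimilarityEval's Hausdorff and average Hausdorff distances to two text fields.
; A local AverageHausdorfDist function, not called by RefreshText, sums both directions' mean nearest-point 2D distances by brute force, capping each at a fixed maximum.
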(event Custom|RefreshText
  (Variables|Default|SetNotEmpty false)
  (Utilities|FlowControl|Sequence
    (:then_0
      ;[1 1 1] Get Drawing Points from Boards
      (Utilities|FlowControl|Sequence
        (:then_0
          (Variables|Default|SetLVecArr (Variables|/Game/Whiteboard/BP_Whiteboard.BP_Whiteboard_C|GetDrawArray (Variables|Default|GetCompareBoard1)))
          (Variables|Default|SetRVecArr (Variables|/Game/Whiteboard/BP_Whiteboard.BP_Whiteboard_C|GetDrawArray (Variables|Default|GetCompareBoard2))))
        (:then_1
          (Variables|Default|SetNotEmpty (and (>= (Utilities|Array|Length (Variables|Default|GetLVecArr)) 1) (>= (Utilities|Array|Length (Variables|Default|GetRVecArr)) 1))))))
    (:then_1
      (if (Variables|Default|GetNotEmpty)
        ;[1 1 1] Hausdorff
        (Rendering|Components|TextRender|SetText (Variables|Default|GetHausdorffRes) (Utilities|Text|FormatText "Hausdorff dist : {hausdist}" (Class|SimilarityEvalComponent|HausdorffDist (Variables|Default|GetSimilarityEval) (Variables|Default|GetLVecArr) (Variables|Default|GetRVecArr))))
        ;[1 1 1] Average Hausdorff
        (Rendering|Components|TextRender|SetText (Variables|Default|GetAvgHausdorffRes) (Utilities|Text|FormatText "Average Hausdorff dist : {hausdist}" (Class|SimilarityEvalComponent|AverageHausdorffDist (Variables|Default|GetSimilarityEval) (Variables|Default|GetLVecArr) (Variables|Default|GetRVecArr))))))))

(fn ConstructionScript)

(fn AverageHausdorfDist
  (params (linex :type Array%20of%20Vector%202D%20Structures) (liney :type Array%20of%20Vector%202D%20Structures))
  (Utilities|FlowControl|Sequence
    (:then_0
      (LocalVariables|Setxsize (Utilities|Array|Length linex)))
    (:then_1
      (LocalVariables|Setysize (Utilities|Array|Length liney)))
    (:then_2
      (for _array_element linex
        (LocalVariables|SetMinY 3e+03)
        (for _array_element_2 liney
          (LocalVariables|SetMinY (Math|Float|Min(Float) (Math|Vector|Distance2D(Vector) _array_element _array_element_2) (LocalVariables|GetMinY))))
        (LocalVariables|SetTotY (+ (LocalVariables|GetTotY) (LocalVariables|GetMinY)))))
    (:then_3
      (for _array_element_3 liney
        (LocalVariables|SetMinX 3e+03)
        (for _array_element_4 linex
          (LocalVariables|SetMinX (Math|Float|Min(Float) (Math|Vector|Distance2D(Vector) _array_element_3 _array_element_4) (LocalVariables|GetMinX))))
        (LocalVariables|SetTotX (+ (LocalVariables|GetTotX) (LocalVariables|GetMinX)))))
    (:then_4
      (return (+ (/ (LocalVariables|GetTotX) (Math|Conversions|ToFloat(Integer) (LocalVariables|Getxsize))) (/ (LocalVariables|GetTotY) (Math|Conversions|ToFloat(Integer) (LocalVariables|Getysize))))))))